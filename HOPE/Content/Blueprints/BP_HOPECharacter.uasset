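; Player character Blueprint handling first-layer input and feedback for shooting, reload, aim zoom, dash and ammo switching around HOPECharacter functions.
; A Gate and retriggerable delay loop drives automatic fire, with chained timelines adding recoil pitch.
; An FOV timeline handles aiming and reverses on Tick while reloading, running or wielding the katana, which also blocks gunfire.
; A Footstep overlap maps physical material to a Surface enum.
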(event `Key|LeftMouseButton`
  (params (Key :type "Key Structure"))
  (:`Pressed`
    (if (not (`self.IsOnKATANA`))
      (cast `HOPECharacter` (`GameplayStatics.GetPlayerPawn` 0))
      (if (> (`self.AmmoCount`) 0)
        (`|ExecutionSequence`
          (:`then_0`
            (goto _label :!via `Open`))
          (:`then_1`
            (`/Engine/EditorBlueprintResources/StandardMacros.Gate` true :!label _label
              (:`Exit`
                (`|ExecutionSequence`
                  (:`then_0`
                    (if (not (`self.IsOnKatana`))
                      (`self.Shoot`)
                      (if (and (> (`self.AmmoCount`) 0) (not (`self.IsReloading`)) (not (`self.IsOnKATANA`)))
                        (bind (_direction `_새_트랙_0`) (`Timeline|타임라인_2` :!via `PlayFromStart`)
                          (:`Update`
                            (`self.AddControllerPitchInput` (`PawnMovementComponent.GetPawnOwner` (`self.CharacterMovement`)) (`KismetMathLibrary.FInterpTo` 0.0 -0.04 1.0 `_새_트랙_0`))
                            (bind (_direction_2 `_새_트랙_0_2`) (`Timeline|타임라인_1` :!via `PlayFromStart`)
                              (:`Update`
                                (`self.AddControllerPitchInput` (`PawnMovementComponent.GetPawnOwner` (`self.CharacterMovement`)) (`KismetMathLibrary.FInterpTo` 0.0 0.01 1.0 `_새_트랙_0_2`)))))))))
                  (:`then_1`
                    (`KismetSystemLibrary.RetriggerableDelay` 0.1)
                    (goto _label)))))))
        (elif (not (`self.IsReloading`))
          (`GameplayStatics.PlaySoundAtLocation` "/Game/M4A4_Animated/Sounds/Sound_Packs/Warfare_SFX_Bundle/Gun_Sound_Essentials/Wavs/Dry_shot_1.Dry_shot_1" (0.0 0.0 0.0) (struct) 0.6 1.0 0.0 null null null)))))
  (:`Released`
    (goto _label :!via `Close`)))

(event `InputAction|Reload`
  (params (Key :type "Key Structure"))
  (:`Pressed`
    (if (not (`self.IsReloading`))
      (`self.Reload`)
      (`SkeletalMeshComponent.PlayAnimation` (`self.Weapon`) "/Game/Gun/Gun_Animations/Gun_Reload.Gun_Reload" false))))

(event `Key|RightMouseButton`
  (params (Key :type "Key Structure"))
  (:`Pressed`
    (if (`self.IsOnKATANA`)
      _
      (elif (not (`self.IsReloading`))
        (`GameplayStatics.PlaySoundAtLocation` "/Game/M4A4_Animated/Sounds/Sound_Packs/Bonus_Sounds/Wavs/M4_Draw.M4_Draw" (0.0 0.0 0.0) (struct) 1.0 1.0 0.7 null null null)
        (bind (_direction `_새_트랙_0`) (`Timeline|타임라인_0` :!via `PlayFromStart` :!label _label_2)
          (:`Update`
            (`CameraComponent.SetFieldOfView` (`self.Camera`) `_새_트랙_0`))))))
  (:`Released`
    (if (not (`self.IsOnKATANA`))
      (`GameplayStatics.PlaySoundAtLocation` "/Game/M4A4_Animated/Sounds/Sound_Packs/Bonus_Sounds/Wavs/AKM_Holster.AKM_Holster" (0.0 0.0 0.0) (struct) 1.0 1.0 0.5 null null null)
      (goto _label_2 :!via `Reverse`))))

(event `InputAction|Dash`
  (params (Key :type "Key Structure"))
  (:`Pressed`
    (`self.Dash`)
    (if (and (== (`self.CountDashCooltime`) 0.0) (not (`NavMovementComponent.IsFalling` (`self.CharacterMovement`))))
      (`GameplayStatics.PlaySoundAtLocation` "/Game/M4A4_Animated/Sounds/Sound_Packs/Bullet_Impacts_Flybys_Pro/Wavs/Bullet_Flybys/Bullet_Flyby_8.Bullet_Flyby_8" (0.0 0.0 0.0) (struct) 0.6 1.0 0.1 null null null)
      (`AddComponent|NODE_AddNiagaraComponent-0`))))

(event `self.ReceiveTick`
  (params (DeltaSeconds :type "Float (single-precision)"))
  (if (or (`self.IsReloading`) (`self.IsRunning`) (`self.IsOnKATANA`))
    (goto _label_2 :!via `Reverse`)))

(event `InputAction|ChangeAmmo`
  (params (Key :type "Key Structure"))
  (:`Pressed`
    (`self.ChangeAmmo`)
    (if (and (== (`self.CountAmmoCooltime`) 0.0) (not (`self.IsOnKatana`)))
      (`GameplayStatics.PlaySoundAtLocation` "/Game/M4A4_Animated/Sounds/Sound_Packs/Bullet_Impacts_Flybys_Pro/Wavs/Dirt/Dirt_7.Dirt_7" (0.0 0.0 0.0) (struct) 1.0 1.0 0.0 null null null))))

(event `self.Footstep.OnComponentBeginOverlap`
  (params (OverlappedComponent :type "PrimitiveComponent Object Reference") (OtherActor :type "Actor Object Reference") (OtherComp :type "PrimitiveComponent Object Reference") (OtherBodyIndex :type Integer) (bFromSweep :type Boolean) (SweepResult :type "HitResult Structure (by ref)"))
  (switch `EPhysicalSurface` (`PhysicalMaterial.SurfaceType` (`MaterialInterface.GetPhysicalMaterial` (`PrimitiveComponent.GetMaterial` (`.HitComponent` (`GameplayStatics.BreakHitResult` SweepResult)) 0)))
    (:`SurfaceType_Default`
      (set `self.Surface` "NewEnumerator0"))
    (:`SurfaceType2`
      (set `self.Surface` "NewEnumerator6"))
    (:`SurfaceType4`
      (set `self.Surface` "NewEnumerator3"))
    (:`SurfaceType5`
      (set `self.Surface` "NewEnumerator2"))
    (:`SurfaceType6`
      (set `self.Surface` "NewEnumerator4"))
    (:`SurfaceType7`
      (set `self.Surface` "NewEnumerator1"))
    (:`SurfaceType8`
      (set `self.Surface` "NewEnumerator7"))))

(fn `UserConstructionScript`)