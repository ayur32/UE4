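; BP_BullMech is an AI-controlled bull mech enemy that damages and knocks back what it hits.
; Leg and Head overlaps damage any actor, the Head harder, then launch a HOPECharacter away from the mech, with extra lift from the Head.
; When damaged with IsDeath set, it stops its AI brain logic and calls Death.
; It then plays staged EMP and explosion sounds with particles before destroying itself.
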(event `self.Leg.OnComponentBeginOverlap`
  (params (OverlappedComponent :type "PrimitiveComponent Object Reference") (OtherActor :type "Actor Object Reference") (OtherComp :type "PrimitiveComponent Object Reference") (OtherBodyIndex :type Integer) (bFromSweep :type Boolean) (SweepResult :type "HitResult Structure (by ref)"))
  (`GameplayStatics.ApplyDamage` OtherActor 100.0)
  (bind _ashopecharacter (cast `HOPECharacter` OtherActor))
  (`self.LaunchCharacter` _ashopecharacter (* (- (`self.K2_GetActorLocation` _ashopecharacter) (`self.K2_GetActorLocation`)) 7.0) false false)
  (`KismetSystemLibrary.PrintString` "Leg"))

(event `self.Head.OnComponentBeginOverlap`
  (params (OverlappedComponent :type "PrimitiveComponent Object Reference") (OtherActor :type "Actor Object Reference") (OtherComp :type "PrimitiveComponent Object Reference") (OtherBodyIndex :type Integer) (bFromSweep :type Boolean) (SweepResult :type "HitResult Structure (by ref)"))
  (`GameplayStatics.ApplyDamage` OtherActor 300.0)
  (bind _ashopecharacter (cast `HOPECharacter` OtherActor))
  (bind _returnvalue (`self.K2_GetActorLocation` _ashopecharacter))
  (`self.LaunchCharacter` _ashopecharacter (+ (* (- _returnvalue (`self.K2_GetActorLocation`)) 5.0) (0.0 0.0 500.0)) false false)
  (`GameplayStatics.PlaySoundAtLocation` null _returnvalue (struct) 1.0 1.0 0.0 "/Game/M4A4_Animated/Sounds/Attunation/CasingAttunation.CasingAttunation" null null)
  (`KismetSystemLibrary.PrintString` "Head"))

(event `self.ReceiveAnyDamage`
  (params (Damage :type "Float (single-precision)") (DamageType :type "DamageType Object Reference") (InstigatedBy :type "Controller Object Reference") (DamageCauser :type "Actor Object Reference"))
  (bind _returnvalue (`AIBlueprintHelperLibrary.GetAIController` (`self.GetController`)))
  (if (`self.IsDeath`)
    (`AddComponent|NODE_AddBehaviorTreeComponent-0` :`self` _returnvalue)
    (`BrainComponent.StopLogic` (`AIController.BrainComponent` _returnvalue) "")
    (`self.Death`)
    (`AddComponent|NODE_AddParticleSystemComponent-2`)
    (`AddComponent|NODE_AddParticleSystemComponent-4`)
    (`GameplayStatics.PlaySoundAtLocation` "/Game/M4A4_Animated/Sounds/Sound_Packs/Warfare_SFX_Bundle/Explosion_Sounds_Pro/Wavs/EMP_Explosion_2.EMP_Explosion_2" (`self.K2_GetActorLocation`) (struct) 5.0 1.0 0.0 "/Game/M4A4_Animated/Sounds/Attunation/Default.Default" null null)
    (`KismetSystemLibrary.Delay` 1.0)
    (`AddComponent|NODE_AddParticleSystemComponent-0`)
    (`AddComponent|NODE_AddParticleSystemComponent-1`)
    (`GameplayStatics.PlaySoundAtLocation` "/Game/M4A4_Animated/Sounds/Sound_Packs/Warfare_SFX_Bundle/Explosion_Sounds_Pro/Wavs/Explosion_Raw_1.Explosion_Raw_1" (`self.K2_GetActorLocation`) (struct) 5.0 1.0 0.0 "/Game/M4A4_Animated/Sounds/Attunation/Default.Default" null null)
    (`KismetSystemLibrary.Delay` 5.0)
    (`self.K2_DestroyActor`)))

(fn `UserConstructionScript`)