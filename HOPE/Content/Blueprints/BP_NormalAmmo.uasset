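; BP_NormalAmmo is an ammo actor that plays surface-specific impact effects when it hits something.
; On Hit, it reads the surface type from the physical material of the hit component's first material.
; A switch covers skin, metal, grass, rock, ground, wood and snow, each adding a particle component and playing an impact sound at the hit location.
; BeginPlay, overlap, Tick and the construction script are empty.
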(event `self.ReceiveHit`
  (params (MyComp :type "PrimitiveComponent Object Reference") (Other :type "Actor Object Reference") (OtherComp :type "PrimitiveComponent Object Reference") (bSelfMoved :type Boolean) (HitLocation :type "Vector Structure") (HitNormal :type "Vector Structure") (NormalImpulse :type "Vector Structure") (Hit :type "HitResult Structure (by ref)"))
  (switch `EPhysicalSurface` (`PhysicalMaterial.SurfaceType` (`MaterialInterface.GetPhysicalMaterial` (`PrimitiveComponent.GetMaterial` (`.HitComponent` (`GameplayStatics.BreakHitResult` Hit)) 0)))
    (:`SurfaceType1`
      (`AddComponent|NODE_AddParticleSystemComponent-5`)
      (`GameplayStatics.PlaySoundAtLocation` "/Game/M4A4_Animated/Sounds/Sound_Packs/Bullet_Impacts_Flybys_Pro/Wavs/Body_Flesh/Body_Flesh_10.Body_Flesh_10" HitLocation (struct) 2.0 1.0 0.0 "/Game/M4A4_Animated/Sounds/Attunation/CasingAttunation.CasingAttunation" null null))
    (:`SurfaceType2`
      (`AddComponent|NODE_AddParticleSystemComponent-0`)
      (`GameplayStatics.PlaySoundAtLocation` "/Game/M4A4_Animated/Sounds/Sound_Packs/Bullet_Impacts_Flybys_Pro/Wavs/Metal_Light/Metal_Light_4.Metal_Light_4" HitLocation (struct) 2.0 1.0 0.0 "/Game/M4A4_Animated/Sounds/Attunation/CasingAttunation.CasingAttunation" null null))
    (:`SurfaceType4`
      (`AddComponent|NODE_AddParticleSystemComponent-2`)
      (`GameplayStatics.PlaySoundAtLocation` "/Game/M4A4_Animated/Sounds/Sound_Packs/Bullet_Impacts_Flybys_Pro/Wavs/Grass/Grass_4.Grass_4" HitLocation (struct) 2.0 1.0 0.0 "/Game/M4A4_Animated/Sounds/Attunation/CasingAttunation.CasingAttunation" null null))
    (:`SurfaceType5`
      (`AddComponent|NODE_AddParticleSystemComponent-4`)
      (`GameplayStatics.PlaySoundAtLocation` "/Game/M4A4_Animated/Sounds/Sound_Packs/Bullet_Impacts_Flybys_Pro/Wavs/Rock/Rock_7.Rock_7" HitLocation (struct) 2.0 1.0 0.0 "/Game/M4A4_Animated/Sounds/Attunation/CasingAttunation.CasingAttunation" null null))
    (:`SurfaceType6`
      (`AddComponent|NODE_AddParticleSystemComponent-3`)
      (`GameplayStatics.PlaySoundAtLocation` "/Game/M4A4_Animated/Sounds/Sound_Packs/Bullet_Impacts_Flybys_Pro/Wavs/Grass/Grass_1.Grass_1" HitLocation (struct) 2.0 1.0 0.0 "/Game/M4A4_Animated/Sounds/Attunation/CasingAttunation.CasingAttunation" null null))
    (:`SurfaceType7`
      (`AddComponent|NODE_AddParticleSystemComponent-1`)
      (`GameplayStatics.PlaySoundAtLocation` "/Game/M4A4_Animated/Sounds/Sound_Packs/Bullet_Impacts_Flybys_Pro/Wavs/Wood_Heavy/Wood_Heavy_1.Wood_Heavy_1" HitLocation (struct) 2.0 1.0 0.0 "/Game/M4A4_Animated/Sounds/Attunation/CasingAttunation.CasingAttunation" null null))
    (:`SurfaceType8`
      (`AddComponent|NODE_AddParticleSystemComponent-6`)
      (`GameplayStatics.PlaySoundAtLocation` "/Game/M4A4_Animated/Sounds/Sound_Packs/Bullet_Impacts_Flybys_Pro/Wavs/Snow/Snow_8.Snow_8" HitLocation (struct) 2.0 1.0 0.0 "/Game/M4A4_Animated/Sounds/Attunation/CasingAttunation.CasingAttunation" null null))))

(fn `UserConstructionScript`)