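; Behavior Tree task for the BullMech AI that picks a chase destination near the player and switches the mech into chasing.
; It writes a random navigable point within a small radius of player character 0 to a Blackboard vector key.
; It then flags the BULLMECH_BP pawn as chasing, fires its chase event, sets a Blackboard bool and finishes successfully.
; A failed pawn cast leaves the task unfinished.
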(event `self.ReceiveExecuteAI`
  (params (OwnerController :type "AIController Object Reference") (ControlledPawn :type "Pawn Object Reference"))
  (`BTFunctionLibrary.SetBlackboardValueAsVector` (`self.Vector`) (`NavigationSystemV1.K2_GetRandomLocationInNavigableRadius` (`Actor.K2_GetActorLocation` (`GameplayStatics.GetPlayerCharacter` 0)) 100.0 null null))
  (bind _asbullmech_bp (cast `/Game/BullMech/BLUEPRINTS/BULLMECH_BP` ControlledPawn))
  (set `/Game/BullMech/BLUEPRINTS/BULLMECH_BP.IsChasing` true _asbullmech_bp)
  (`/Game/BullMech/BLUEPRINTS/BULLMECH_BP.Event Chasing` _asbullmech_bp)
  (`BTFunctionLibrary.SetBlackboardValueAsBool` (`self.Boolean`) true)
  (`self.FinishExecute` true))