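; BULLMECH_BP is the BullMech boss character, handling its wake-up, chase speed, health and death.
; Chasing toggles movement speed and acceleration from IsChasing, while Awake powers the boss on.
; Front and Back overlap volumes set position flags, intended for the AnimBP to pick attack animations.
; AnyDamage reduces and prints HP; at zero it stops AI logic, disables collision, plays a death montage and destroys the actor after a delay.
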(event `Event Chasing`
  (bind _charactermovement (`self.CharacterMovement`))
  ;[1 1 1] Modify Character movement component to speed up while chasing
  (if (`self.IsChasing`)
    (set `CharacterMovementComponent.MaxAcceleration` 1400.0 _charactermovement)
    (set `CharacterMovementComponent.MaxWalkSpeed` 1400.0 _charactermovement)
    (else
      (set `CharacterMovementComponent.MaxAcceleration` 800.0 _charactermovement)
      (set `CharacterMovementComponent.MaxWalkSpeed` 800.0 _charactermovement))))

(event `Event Awake`
  ;[1 1 1] Powering On the boss!
  (set `self.IsChasing` false)
  (set `self.IsAwake` true))

(event `self.Front.OnComponentBeginOverlap`
  (params (OverlappedComponent :type "PrimitiveComponent Object Reference") (OtherActor :type "Actor Object Reference") (OtherComp :type "PrimitiveComponent Object Reference") (OtherBodyIndex :type Integer) (bFromSweep :type Boolean) (SweepResult :type "HitResult Structure (by ref)"))
  ;[1 1 1] Attack events to send to AnimBP to execute attacks animations
  (set `self.IsInFront` true))

(event `self.ReceiveAnyDamage`
  (params (Damage :type "Float (single-precision)") (DamageType :type "DamageType Object Reference") (InstigatedBy :type "Controller Object Reference") (DamageCauser :type "Actor Object Reference"))
  (bind _returnvalue (`AIBlueprintHelperLibrary.GetAIController` (`self.GetController`)))
  (set `self.CurrentHP` (- (`self.CurrentHP`) Damage))
  (`KismetSystemLibrary.PrintString` (`KismetStringLibrary.Conv_DoubleToString` (`self.CurrentHP`)))
  (if (<= (`self.CurrentHP`) 0.0)
    (`AddComponent|NODE_AddBehaviorTreeComponent-0` :`self` _returnvalue)
    (`BrainComponent.StopLogic` (`AIController.BrainComponent` _returnvalue) "")
    (`PrimitiveComponent.SetCollisionEnabled` (`self.Mesh`) "NoCollision")
    (`PrimitiveComponent.SetCollisionEnabled` (`self.CapsuleComponent`) "NoCollision")
    (`|PlayMontage` (`self.Mesh`) "/Game/BullMech/ANIMATIONS/BullMech_Death_Montage.BullMech_Death_Montage"
      (:`then`
        (`KismetSystemLibrary.Delay` 5.0)
        (`self.K2_DestroyActor`)))))

(event `self.Back.OnComponentBeginOverlap`
  (params (OverlappedComponent :type "PrimitiveComponent Object Reference") (OtherActor :type "Actor Object Reference") (OtherComp :type "PrimitiveComponent Object Reference") (OtherBodyIndex :type Integer) (bFromSweep :type Boolean) (SweepResult :type "HitResult Structure (by ref)"))
  ;[1 1 1] Attack events to send to AnimBP to execute attacks animations
  (set `self.IsInBack` true))

(event `self.Front.OnComponentEndOverlap`
  (params (OverlappedComponent :type "PrimitiveComponent Object Reference") (OtherActor :type "Actor Object Reference") (OtherComp :type "PrimitiveComponent Object Reference") (OtherBodyIndex :type Integer))
  ;[1 1 1] Attack events to send to AnimBP to execute attacks animations
  (set `self.IsInFront` false))

(event `self.Back.OnComponentEndOverlap`
  (params (OverlappedComponent :type "PrimitiveComponent Object Reference") (OtherActor :type "Actor Object Reference") (OtherComp :type "PrimitiveComponent Object Reference") (OtherBodyIndex :type Integer))
  ;[1 1 1] Attack events to send to AnimBP to execute attacks animations
  (set `self.IsInBack` false))

(fn `UserConstructionScript`)